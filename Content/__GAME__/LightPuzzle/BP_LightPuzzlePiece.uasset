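; Light puzzle piece actor whose point light changes color each time it is used.
; OnUse increments a color index that wraps back to zero after the fourth state, then calls UpdateLightColor.
; UpdateLightColor maps the index to a fixed white, green, red-orange or blue color on the PointLight.
; The file holds no solution check, only the color cycling.
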(event EventBeginPlay)

(event Collision|EventActorBeginOverlap
  (params (OtherActor :type Actor%20Object%20Reference)))

(event EventTick
  (params (DeltaSeconds :type Float%20%28single-precision%29)))

(event EventOnUse
  (params (Actor :type Actor%20Object%20Reference))
  (bind _result (Math|Integer|IncrementInt (Variables|Default|Getcolor%20index))
    (:%20%20
      (if (<= _result 3)
        _
        (else
          (Variables|Default|Setcolor%20index 0)))
      (CallFunction|UpdateLightColor))))

(fn ConstructionScript)

(fn UpdateLightColor
  (switch int (Variables|Default|Getcolor%20index)
    (:0
      (Rendering|Components|Light|SetLightColor (Variables|Default|GetPointLight) "(R=0.987301,G=1.000000,B=0.934119,A=1.000000)" true))
    (:1
      (Rendering|Components|Light|SetLightColor (Variables|Default|GetPointLight) "(R=0.036923,G=1.000000,B=0.179031,A=1.000000)" true))
    (:2
      (Rendering|Components|Light|SetLightColor (Variables|Default|GetPointLight) "(R=1.000000,G=0.195490,B=0.025443,A=1.000000)" true))
    (:3
      (Rendering|Components|Light|SetLightColor (Variables|Default|GetPointLight) "(R=0.046377,G=0.207319,B=1.000000,A=1.000000)" true))))