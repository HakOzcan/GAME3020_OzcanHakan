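; Light puzzle door that slides open when its OnUse event is triggered by a BP_PuzzleChecker.
; OnUse opens a Gate on Tick, which then moves Door2 toward the OPenPOs component's world location at constant speed via VInterpToConstant.
; The gate is never closed, so there is no closing path.
; An older FlipFlop and timeline yaw-rotation opening is left disconnected and never runs.
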(event EventBeginPlay)

(event Collision|EventActorBeginOverlap
  (params (OtherActor :type Actor%20Object%20Reference)))

(event EventOnUse
  (params (Actor :type Actor%20Object%20Reference))
  (Utilities|Casting|CastToBP_PuzzleChecker Actor)
  (Utilities|FlowControl|Gate true) ; enters at Open
)

(event EventTick
  (params (DeltaSeconds :type Float%20%28single-precision%29))
  (Utilities|FlowControl|Gate true
    (:Exit
      (Transformation|SetWorldLocation (Variables|Default|GetDoor_2) (Math|Interpolation|VInterptoConstant (Transformation|GetWorldLocation (Variables|Default|GetDoor_2)) (Transformation|GetWorldLocation (Variables|Default|GetOPen%20POs)) DeltaSeconds 6e+01) false false))))

(fn ConstructionScript)