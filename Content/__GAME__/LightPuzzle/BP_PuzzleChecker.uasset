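; Light puzzle checker that, when used, tests whether the puzzle pieces show the correct color code and opens a door if they do.
; It compares each piece's ColorIndex against the ColorCode entry at the same index, stopping at the first mismatch.
; A match sends OnUse to DoorToOpen through Use_Interface, guarded by a DoOnce so it fires a single time.
; A mismatch resets every piece to color index zero and refreshes its light.
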(event EventBeginPlay)

(event Collision|EventActorBeginOverlap
  (params (OtherActor :type Actor%20Object%20Reference)))

(event EventTick
  (params (DeltaSeconds :type Float%20%28single-precision%29)))

(event EventOnUse
  (params (Actor :type Actor%20Object%20Reference))
  (Variables|Default|Setis%20correct? true)
  (bind (_array_element _array_index) (Utilities|Array|ForEachLoopwithBreak (Variables|Default|Getpuzzle%20pieces) :!label _label)
    (:LoopBody
      (if (!= (Variables|/Game/__GAME__/LightPuzzle/BP_LightPuzzlePiece.BP_LightPuzzlePiece_C|Getcolor%20index _array_element) (Utilities|Array|Get(acopy) (Variables|Default|Getcolor%20code) _array_index))
        (Variables|Default|Setis%20correct? false)
        (goto _label Break)))
    (:Completed
      (if (Variables|Default|Getis%20correct?)
        (Utilities|FlowControl|DoOnce false
          (:Completed
            (bind _door_to_open (Variables|Default|Getdoor%20to%20open)
              (:then
                (if (Utilities|DoesObjectImplementInterface _door_to_open "/Game/__GAME__/LightPuzzle/Use_Interface.Use_Interface_C")
                  (Class|UseInterface|OnUse(Message) _door_to_open self)))
              (:else))))
        (else
          (for _array_element_2 (Variables|Default|Getpuzzle%20pieces)
            (Variables|/Game/__GAME__/LightPuzzle/BP_LightPuzzlePiece.BP_LightPuzzlePiece_C|Setcolor%20index _array_element_2 0)
            (Default|UpdateLightColor _array_element_2)))))))

(fn ConstructionScript)