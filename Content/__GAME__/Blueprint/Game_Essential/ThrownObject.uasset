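; ThrownObject is a one-shot scripted scare or event actor that flings five props when something overlaps its trigger box.
; On the first Box overlap, a DoOnce enables physics on the five objects and applies a large +Y force to knock them away.
; It plays a metal drop sound at the actor, then after a one-second delay plays a dialogue line at the player's location.
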(event OnComponentBeginOverlap(Box)
  (params (OverlappedComponent :type Primitive%20Component%20Object%20Reference) (OtherActor :type Actor%20Object%20Reference) (OtherComp :type Primitive%20Component%20Object%20Reference) (OtherBodyIndex :type Integer) (bFromSweep :type Boolean) (SweepResult :type Hit%20Result%20Structure%20%28by%20ref%29))
  (bind _thrown_object (Variables|Default|GetThrown%20Object))
  (Utilities|FlowControl|DoOnce false
    (:Completed
      (Physics|SetSimulatePhysics _thrown_object true)
      (Physics|AddForce _thrown_object "0.000000,10000000.000000,0.000000" "None" false)
      (Audio|PlaySoundatLocation "/Game/__GAME__/Music/MetalDropOnFloor.MetalDropOnFloor" (Transformation|GetActorLocation) "0, 0, 0" 1.0 1.0 0.0 0 0 0 0)
      (Utilities|FlowControl|Delay 1.0)
      (Audio|PlaySoundatLocation "/Game/__GAME__/Music/L2_Dialogue.L2_Dialogue" (Transformation|GetActorLocation (Game|GetPlayerCharacter 0)) "0, 0, 0" 1.0 1.0 0.0 0 0 0 0))))

(fn ConstructionScript)