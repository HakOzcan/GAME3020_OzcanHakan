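; First-person player character that routes Enhanced Input to movement and flashlight components, with a timeline resizing the capsule for crouch.
; Interact runs both a sphere trace and a camera line trace, messaging hit actors through interfaces.
; A toggleable camera mode adds an overlay widget, post-process and clamped FOV zoom.
; It also reports jump and shoot achievements, plays landing force feedback, defines speed-based head-bob shakes and stores a passcode.
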(event Custom|ShortenPlayerCapsule
  ;[1 1 1] Crouch
  (bind _alpha (Timeline|CapsuleTL Play)
    (:Update
      (Components|Capsule|SetCapsuleHalfHeight (Variables|Default|GetCapsuleComponent) (Math|Float|Lerp 96.0 (Variables|/Game/__GAME__/Blueprint/Game_Essential/Components/BPC_Movement.BPC_Movement_C|GetCrouchHalfHeight (Variables|Default|GetBPC_Movement)) _alpha) true))))

(event Custom|LengthenPlayerCapsule
  ;[1 1 1] Crouch
  (bind _alpha (Timeline|CapsuleTL Reverse)
    (:Update
      (Components|Capsule|SetCapsuleHalfHeight (Variables|Default|GetCapsuleComponent) (Math|Float|Lerp 96.0 (Variables|/Game/__GAME__/Blueprint/Game_Essential/Components/BPC_Movement.BPC_Movement_C|GetCrouchHalfHeight (Variables|Default|GetBPC_Movement)) _alpha) true))))

(event Input|EnhancedActionEvents|EnhancedInputActionIA_Interact
  (params (ActionValue :type Boolean) (ElapsedSeconds :type Float%20%28double-precision%29) (TriggeredSeconds :type Float%20%28double-precision%29) (InputAction :type Input%20Action%20Object%20Reference :default "/Game/__GAME__/Input/Actions/IA_Interact.IA_Interact"))
  (bind _firstpersoncameracomponent (Variables|Default|GetFirstPersonCameraComponent))
  (bind _returnvalue (Transformation|GetWorldLocation _firstpersoncameracomponent))
  ;[1 1 1] Use Event
  (bind (_outhit _returnvalue_2) (Collision|LineTraceByChannel _returnvalue (+ _returnvalue (* (Math|Vector|GetForwardVector _firstpersoncameracomponent) 3.5e+02)) "TraceTypeQuery1" false 0 "ForDuration" true "(R=1.000000,G=0.000000,B=0.000000,A=1.000000)" "(R=0.000000,G=1.000000,B=0.000000,A=1.000000)" 1.0))
  (if _returnvalue_2
    (if (Utilities|DoesObjectImplementInterface (.HitActor (Collision|BreakHitResult _outhit)) "/Game/__GAME__/LightPuzzle/Use_Interface.Use_Interface_C")
      (Class|UseInterface|OnUse(Message) (.HitActor (Collision|BreakHitResult _outhit)) self))))

(event Input|EnhancedActionEvents|EnhancedInputActionIA_Shoot
  (params (ActionValue :type Boolean) (ElapsedSeconds :type Float%20%28double-precision%29) (TriggeredSeconds :type Float%20%28double-precision%29) (InputAction :type Input%20Action%20Object%20Reference :default "/Game/__GAME__/Input/Actions/IA_Shoot.IA_Shoot"))
  (bind _returnvalue (Subsystems|GetAchievementSubSystem))
  (Class|AchievementSubSystem|AddAchievementProgress _returnvalue "Shoot" 1.0)
  (Class|AchievementSubSystem|AddAchievementProgress _returnvalue "Shoot_100" 1.0)
  (Class|AchievementSubSystem|AddAchievementProgress _returnvalue "Shoot_1000" 1.0))

(event Input|EnhancedActionEvents|EnhancedInputActionIA_Sprint
  (params (ActionValue :type Boolean) (ElapsedSeconds :type Float%20%28double-precision%29) (TriggeredSeconds :type Float%20%28double-precision%29) (InputAction :type Input%20Action%20Object%20Reference :default "/Game/__GAME__/Input/Actions/IA_Sprint.IA_Sprint"))
  (bind _bpc_movement (Variables|Default|GetBPC_Movement))
  ;[1 1 1] Sprint
  (:Triggered
    (Default|StartSprint _bpc_movement :!label _label))
  (:Started
    (goto _label))
  (:Ongoing
    (goto _label))
  (:Completed
    (Default|StopSprint _bpc_movement)))

(event Input|EnhancedActionEvents|EnhancedInputActionIA_Crouch
  (params (ActionValue :type Boolean) (ElapsedSeconds :type Float%20%28double-precision%29) (TriggeredSeconds :type Float%20%28double-precision%29) (InputAction :type Input%20Action%20Object%20Reference :default "/Game/__GAME__/Input/Actions/IA_Crouch.IA_Crouch"))
  (bind _bpc_movement (Variables|Default|GetBPC_Movement))
  ;[1 1 1] Crouch
  (:Started
    (if (Variables|/Game/__GAME__/Blueprint/Game_Essential/Components/BPC_Movement.BPC_Movement_C|GetisCrouching _bpc_movement)
      (Default|StopCrouch _bpc_movement)
      (else
        (Default|StartCrouch _bpc_movement)))))

(event Input|EnhancedActionEvents|EnhancedInputActionIA_Interact
  (params (ActionValue :type Boolean) (ElapsedSeconds :type Float%20%28double-precision%29) (TriggeredSeconds :type Float%20%28double-precision%29) (InputAction :type Input%20Action%20Object%20Reference :default "/Game/__GAME__/Input/Actions/IA_Interact.IA_Interact"))
  (bind _returnvalue (Transformation|GetActorLocation))
  ;[1 1 1] Interact Logic
  (bind (_outhit _returnvalue_2) (Collision|SphereTraceByChannel _returnvalue _returnvalue 1e+02 "TraceTypeQuery1" false 0 "ForDuration"))
  (if _returnvalue_2
    (Class|BPIInteractInterface|InteractEvent(Message) (.HitActor (Collision|BreakHitResult _outhit)))))

(event Input|EnhancedActionEvents|EnhancedInputActionIA_FlashLight
  (params (ActionValue :type Boolean) (ElapsedSeconds :type Float%20%28double-precision%29) (TriggeredSeconds :type Float%20%28double-precision%29) (InputAction :type Input%20Action%20Object%20Reference :default "/Game/__GAME__/Input/Actions/IA_FlashLight.IA_FlashLight"))
  ;[1 1 1] Flash Light
  (:Started
    (Default|ToggleFlashLight (Variables|Default|GetBPC_Flashlight))))

(event Input|EnhancedActionEvents|EnhancedInputActionIA_Camera
  (params (ActionValue :type Boolean) (ElapsedSeconds :type Float%20%28double-precision%29) (TriggeredSeconds :type Float%20%28double-precision%29) (InputAction :type Input%20Action%20Object%20Reference :default "/Game/__GAME__/Input/Actions/IA_Camera.IA_Camera"))
  (bind _cameraref (Variables|Default|GetCameraRef))
  ;[1 1 1] Camera
  (:Started
    (if (Variables|Default|GetisCameraOn)
      (Variables|Default|SetisCameraOn false)
      (Widget|RemovefromParent _cameraref)
      (Camera|SetFieldOfView (Variables|Default|GetFirstPersonCameraComponent) (Variables|Default|GetmaxFOV))
      (Default|CallTogglePostProcessVolume false)
      (else
        (Variables|Default|SetisCameraOn true)
        (UserInterface|Viewport|AddtoViewport _cameraref 0)
        (Default|CallTogglePostProcessVolume true)))))

(event Input|EnhancedActionEvents|EnhancedInputActionIA_CameraZoomIn
  (params (ActionValue :type Boolean) (ElapsedSeconds :type Float%20%28double-precision%29) (TriggeredSeconds :type Float%20%28double-precision%29) (InputAction :type Input%20Action%20Object%20Reference :default "/Game/__GAME__/Input/Actions/IA_CameraZoomIn.IA_CameraZoomIn"))
  (bind _firstpersoncameracomponent (Variables|Default|GetFirstPersonCameraComponent))
  ;[1 1 1] Camera
  (:Started
    (if (Variables|Default|GetisCameraOn)
      (Camera|SetFieldOfView _firstpersoncameracomponent (Math|Float|Clamp(Float) (+ (Variables|/Script/Engine.CameraComponent|GetFieldOfView _firstpersoncameracomponent) -5.0) (Variables|Default|GetminFOV) (Variables|Default|GetmaxFOV))))))

(event Input|EnhancedActionEvents|EnhancedInputActionIA_CameraZoomOut
  (params (ActionValue :type Boolean) (ElapsedSeconds :type Float%20%28double-precision%29) (TriggeredSeconds :type Float%20%28double-precision%29) (InputAction :type Input%20Action%20Object%20Reference :default "/Game/__GAME__/Input/Actions/IA_CameraZoomOut.IA_CameraZoomOut"))
  (bind _firstpersoncameracomponent (Variables|Default|GetFirstPersonCameraComponent))
  ;[1 1 1] Camera
  (:Started
    (if (Variables|Default|GetisCameraOn)
      (Camera|SetFieldOfView _firstpersoncameracomponent (Math|Float|Clamp(Float) (+ (Variables|/Script/Engine.CameraComponent|GetFieldOfView _firstpersoncameracomponent) 5.0) (Variables|Default|GetminFOV) (Variables|Default|GetmaxFOV))))))

(event EventOnLanded
  (params (Hit :type Hit%20Result%20Structure%20%28by%20ref%29))
  (Game|Feedback|ClientPlayForceFeedback (Class|MyBlueprintFunctionLibrary|GetActivePlayerController) "/Game/__GAME__/Input/Force_Feedback/FF_Landing.FF_Landing" "None" false false false)
  (Class|AutoSaveSubsystem|IncrementJumpCount (Subsystems|GetAutoSaveSubsystem)))

(event EventOnJumped
  (bind _returnvalue (Subsystems|GetAchievementSubSystem))
  (Class|AchievementSubSystem|AddAchievementProgress _returnvalue "Jump" 1.0)
  (Class|AchievementSubSystem|AddAchievementProgress _returnvalue "Jump_100" 1.0)
  (Class|AchievementSubSystem|AddAchievementProgress _returnvalue "Jump_200" 1.0))

(event EventBeginPlay
  (Utilities|FlowControl|Sequence
    (:then_0
      (Default|Initialize (Variables|Default|GetBPC_Movement) self))
    (:then_1
      (Default|Initialize (Variables|Default|GetBPC_Flashlight) self))
    (:then_2
      (bind _returnvalue (UserInterface|CreateWidget "/Game/__GAME__/Blueprint/Game_Essential/UI/WBP_Camera.WBP_Camera_C"))
      (Variables|Default|SetCameraRef _returnvalue)
      (Variables|Default|SetmaxFOV (Variables|/Script/Engine.CameraComponent|GetFieldOfView (Variables|Default|GetFirstPersonCameraComponent))))))

(fn ConstructionScript)

(fn HeadBob
  (bind _returnvalue (Transformation|GetVelocity))
  (bind _returnvalue_2 (Transformation|GetVelocity))
  (bind _returnvalue_3 (Game|GetPlayerController 0))
  (bind _charactermovement (Variables|Character|GetCharacterMovement))
  (bind _returnvalue_4 (Math|Vector|VectorLength _returnvalue))
  (bind _returnvalue_5 (Math|Vector|VectorLength _returnvalue_2))
  (bind _maxwalkspeed (Variables|/Script/Engine.CharacterMovementComponent|GetMaxWalkSpeed _charactermovement))
  (bind _returnvalue_6 (Math|Float|MapRangeClamped _returnvalue_4 0.0 _maxwalkspeed 0.0 1.0))
  (if (and (>= _returnvalue_5 (Variables|/Game/__GAME__/Blueprint/Game_Essential/Components/BPC_Movement.BPC_Movement_C|GetWalkSpeed (Variables|Default|GetBPC_Movement))) (not (AI|Components|NavMovement|IsFalling (Variables|Character|GetCharacterMovement))))
    (if (and (>= _returnvalue_5 (Variables|/Game/__GAME__/Blueprint/Game_Essential/Components/BPC_Movement.BPC_Movement_C|GetSprintSpeed (Variables|Default|GetBPC_Movement))) (not (AI|Components|NavMovement|IsFalling (Variables|Character|GetCharacterMovement))))
      (Game|Feedback|ClientStartCameraShake _returnvalue_3 "/Game/__GAME__/Blueprint/Game_Essential/CameraShake/CS_HeadBob_Run.CS_HeadBob_Run_C" _returnvalue_6 "CameraLocal" "0, 0, 0")
      (else
        (Game|Feedback|ClientStartCameraShake _returnvalue_3 "/Game/__GAME__/Blueprint/Game_Essential/CameraShake/CS_HeadBob_Walk.CS_HeadBob_Walk_C" _returnvalue_6 "CameraLocal" "0, 0, 0")))))

(fn SetPlayerPasscode
  (params (NewPasscode :type String))
  (Variables|Default|SetPlayerPasscode NewPasscode))