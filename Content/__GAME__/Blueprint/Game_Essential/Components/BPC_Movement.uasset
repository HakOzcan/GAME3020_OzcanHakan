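; Movement component that gives the player character stamina-limited sprinting and crouching by switching its max walk speed.
; Looping named timers drain stamina while sprinting, ending the sprint at minimum stamina or near standstill, and refill it after a retriggerable delay.
; Crouching cancels the sprint timer and calls BP_C_Game to resize the capsule, while starting a sprint first stands the player up.
; Stamina values print on screen as they change.
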(event Custom|StartSprint
  ;[1 1 1] Sprint
  (if (Variables|Default|GetisCrouching)
    (CallFunction|StopCrouch))
  (if (and (> (Variables|Default|GetCurrentStamina) (Variables|Default|GetMinStamina)) (> (Math|Vector|VectorLength (Transformation|GetVelocity (Variables|Default|GetPlayerRef))) 1e+01))
    (Utilities|Time|ClearTimerbyFunctionName 0 "RegenerateStamina")
    (CallFunction|SetPlayerMaxWalkSpeed (Variables|Default|GetSprintSpeed))
    (Utilities|Time|SetTimerbyFunctionName 0 "SprintTimer" 0.1 true)))

(event Custom|SprintTimer
  ;[1 1 1] Sprint
  (if (> (Math|Vector|VectorLength (Transformation|GetVelocity (Variables|Default|GetPlayerRef))) 1e+01)
    (bind _output_get (Variables|Default|SetCurrentStamina (Math|Float|Clamp(Float) (- (Variables|Default|GetCurrentStamina) 1.0) (Variables|Default|GetMinStamina) (Variables|Default|GetMaxStamina))))
    (Development|PrintString (Utilities|String|ToString(Float) _output_get) true true "(R=1.000000,G=0.000000,B=0.139645,A=1.000000)")
    (if (<= (Variables|Default|GetCurrentStamina) (Variables|Default|GetMinStamina))
      (CallFunction|StopSprint))
    (else
      (CallFunction|StopSprint))))

(event Custom|StopSprint
  ;[1 1 1] Sprint
  (if (not (Variables|Default|GetisCrouching))
    (Utilities|Time|ClearTimerbyFunctionName 0 "SprintTimer")
    (CallFunction|SetPlayerMaxWalkSpeed (Variables|Default|GetWalkSpeed))
    (Utilities|FlowControl|RetriggerableDelay 5.0)
    (if (not (Class|KismetSystemLibrary|IsTimerActive 0 "SprintTimer"))
      (Utilities|Time|SetTimerbyFunctionName 0 "RegenerateStamina" 0.03 true))))

(event Custom|RegenerateStamina
  ;[1 1 1] Sprint
  (bind _output_get (Variables|Default|SetCurrentStamina (Math|Float|Clamp(Float) (+ (Variables|Default|GetCurrentStamina) 1.0) (Variables|Default|GetMinStamina) (Variables|Default|GetMaxStamina))))
  (Development|PrintString (Utilities|String|ToString(Float) _output_get) true true "(R=0.000000,G=1.000000,B=0.066126,A=1.000000)")
  (if (>= (Variables|Default|GetCurrentStamina) (Variables|Default|GetMaxStamina))
    (Utilities|Time|ClearTimerbyFunctionName 0 "RegenerateStamina")))

(event Custom|StartCrouch
  ;[1 1 1] Crouch
  (Utilities|Time|ClearTimerbyFunctionName 0 "SprintTimer")
  (CallFunction|SetPlayerMaxWalkSpeed (Variables|Default|GetCrouchSpeed))
  (Default|ShortenPlayerCapsule (.AsBP%20C%20Game (Utilities|Casting|CastToBP_C_Game (Variables|Default|GetPlayerRef))))
  (Variables|Default|SetisCrouching true))

(event Custom|StopCrouch
  ;[1 1 1] Crouch
  (CallFunction|SetPlayerMaxWalkSpeed (Variables|Default|GetWalkSpeed))
  (Default|LengthenPlayerCapsule (.AsBP%20C%20Game (Utilities|Casting|CastToBP_C_Game (Variables|Default|GetPlayerRef))))
  (Variables|Default|SetisCrouching false))

(fn Initialize
  (params (Character :type Character%20Object%20Reference))
  (Variables|Default|SetPlayerRef Character)
  (Variables|/Script/Engine.CharacterMovementComponent|SetMaxWalkSpeed (Variables|/Script/Engine.Character|GetCharacterMovement (Variables|Default|GetPlayerRef)) (Variables|Default|GetWalkSpeed)))

(fn SetPlayerMaxWalkSpeed
  (params (Max%20Walk%20Speed :type Float%20%28single-precision%29))
  (Variables|/Script/Engine.CharacterMovementComponent|SetMaxWalkSpeed (Variables|/Script/Engine.Character|GetCharacterMovement (Variables|Default|GetPlayerRef)) Max%20Walk%20Speed))