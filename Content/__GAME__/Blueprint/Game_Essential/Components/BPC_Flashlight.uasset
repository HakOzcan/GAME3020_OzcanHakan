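; Actor component that gives the player a battery-powered flashlight.
; Initialize caches the owning player and its FlashLight light component, which ToggleFlashLight shows or hides, turning it on only when charge is above the minimum.
; While lit, a looping function-name timer drains the clamped battery level, switching the light off and clearing itself at the minimum.
; AddBatteryLife restores charge within the same limits.
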(event EventBeginPlay)

(event EventTick
  (params (DeltaSeconds :type Float%20%28single-precision%29)))

(fn ToggleFlashLight
  (bind _flashlightlight (Variables|Default|GetFlashLightLight))
  (if (Variables|/Script/Engine.SceneComponent|GetbVisible _flashlightlight)
    (Rendering|SetVisibility _flashlightlight false false)
    (Utilities|Time|ClearTimerbyFunctionName 0 "DepleteBatteryLife")
    (elif (> (Variables|Default|GetCurrentBatteryLevel) (Variables|Default|GetMinBatteryLevel))
      (Rendering|SetVisibility _flashlightlight true false)
      (Utilities|Time|SetTimerbyFunctionName 0 "DepleteBatteryLife" (Variables|Default|GetDepletionSpeed) true))))

(fn Initialize
  (params (Player :type BP%20C%20Game%20Object%20Reference))
  (bind _output_get (Variables|Default|SetPlayerRef Player))
  (Variables|Default|SetFlashLightLight (Variables|/Game/__GAME__/Blueprint/Game_Essential/BP_C_Game.BP_C_Game_C|GetFlashLight _output_get)))

(fn DepleteBatteryLife
  (bind _output_get (Variables|Default|SetCurrentBatteryLevel (Math|Float|Clamp(Float) (- (Variables|Default|GetCurrentBatteryLevel) (Variables|Default|GetDepletionAmount)) (Variables|Default|GetMinBatteryLevel) (Variables|Default|GetMaxBatteryLevel))))
  (if (<= _output_get (Variables|Default|GetMinBatteryLevel))
    (Rendering|SetVisibility (Variables|Default|GetFlashLightLight) false false)
    (Utilities|Time|ClearTimerbyFunctionName 0 "DepleteBatteryLife")))

(fn AddBatteryLife
  (params (Amount :type Float%20%28double-precision%29))
  (Variables|Default|SetCurrentBatteryLevel (Math|Float|Clamp(Float) (+ (Variables|Default|GetCurrentBatteryLevel) Amount) (Variables|Default|GetMinBatteryLevel) (Variables|Default|GetMaxBatteryLevel))))