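; BPC_Health is an actor component that tracks a health value for its owner.
; RemoveHealth and AddHealth subtract or add an amount to CurrentHealth, clamping the result between MinHealth and MaxHealth.
; It has no active event logic, so health changes only when other code calls these functions, and it broadcasts no death or change notifications.
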(event EventBeginPlay)

(event EventTick
  (params (DeltaSeconds :type Float%20%28single-precision%29)))

(fn RemoveHealth
  (params (Amount :type Float%20%28double-precision%29))
  (Variables|Default|SetCurrentHealth (Math|Float|Clamp(Float) (- (Variables|Default|GetCurrentHealth) Amount) (Variables|Default|GetMinHealth) (Variables|Default|GetMaxHealth))))

(fn AddHealth
  (params (Amount :type Float%20%28double-precision%29))
  (Variables|Default|SetCurrentHealth (Math|Float|Clamp(Float) (+ (Variables|Default|GetCurrentHealth) Amount) (Variables|Default|GetMinHealth) (Variables|Default|GetMaxHealth))))