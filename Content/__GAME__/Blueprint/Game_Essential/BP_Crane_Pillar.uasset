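; Crane pillar for the Room 5 puzzle that reacts when an actor tagged Room5Solution leaves its sphere trigger.
; On end overlap, it snaps that actor to the skeletal mesh's HangingSocket and disables physics simulation on the meshes.
; The attach result is passed as the ShouldMove flag to its own Mover and to the Movers on both entrance doors, which it finds by class.
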(event OnComponentEndOverlap(Sphere)
  (params (OverlappedComponent :type Primitive%20Component%20Object%20Reference) (OtherActor :type Actor%20Object%20Reference) (OtherComp :type Primitive%20Component%20Object%20Reference) (OtherBodyIndex :type Integer))
  (if (Actor|ActorHasTag OtherActor "Room5Solution")
    (bind _returnvalue (Transformation|AttachComponentToComponent OtherActor (Variables|Default|GetSkeletalMesh) "HangingSocket" "SnapToTarget" "SnapToTarget" "KeepRelative" true))
    (Variables|Default|SetShouldMove _returnvalue)
    (Physics|SetSimulatePhysics (Variables|Debug|GetStaticMeshComponent) false)
    (Class|Mover|SetShouldMove (Variables|Default|GetMover) (Variables|Default|GetShouldMove))
    (bind _returnvalue_2 (Actor|GetActorOfClass "/Game/__GAME__/Blueprint/Game_Essential/BP_EntranceDoor_Right.BP_EntranceDoor_Right_C"))
    (bind _output_get (Variables|Default|SetDoorRight _returnvalue_2))
    (Class|Mover|SetShouldMove (Actor|GetComponentbyClass _output_get "/Script/Template.Mover") (Variables|Default|GetShouldMove))
    (bind _returnvalue_3 (Actor|GetActorOfClass "/Game/__GAME__/Blueprint/Game_Essential/BP_EntranceDoor_Left.BP_EntranceDoor_Left_C"))
    (bind _output_get_2 (Variables|Default|SetDoorLeft _returnvalue_3))
    (Class|Mover|SetShouldMove (Actor|GetComponentbyClass _output_get_2 "/Script/Template.Mover") (Variables|Default|GetShouldMove))))

(fn ConstructionScript)