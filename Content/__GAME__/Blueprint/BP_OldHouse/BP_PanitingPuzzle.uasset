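; BP_PanitingPuzzle is a painting puzzle piece that rotates its picture frame when the player character interacts with it.
; A timeline turns the frame 90 degrees in pitch per use, ignoring re-triggers mid-turn, then advances a wrapping position counter.
; Event dispatchers report failure at position three or success at the PuzzleSolved position.
; Box overlap also triggers rotation, though it is marked unused.
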(event OnComponentEndOverlap(Box)
  (params (OverlappedComponent :type Primitive%20Component%20Object%20Reference) (OtherActor :type Actor%20Object%20Reference) (OtherComp :type Primitive%20Component%20Object%20Reference) (OtherBodyIndex :type Integer))
  ;[1 1 1] not using anymore
  (Utilities|Casting|CastToBP_C_Game OtherActor)
  (Variables|Default|Setinrange false))

(event OnComponentBeginOverlap(Box)
  (params (OverlappedComponent :type Primitive%20Component%20Object%20Reference) (OtherActor :type Actor%20Object%20Reference) (OtherComp :type Primitive%20Component%20Object%20Reference) (OtherBodyIndex :type Integer) (bFromSweep :type Boolean) (SweepResult :type Hit%20Result%20Structure%20%28by%20ref%29))
  ;[1 1 1] not using anymore
  (Utilities|Casting|CastToBP_C_Game OtherActor)
  (Variables|Default|Setinrange true)
  (CallFunction|Roataed))

(event Custom|roataed
  ;[1 1 1] roating it
  (if (not (Variables|Default|Getframemoving))
    (Variables|Default|Setframemoving true)
    (bind _rotation (Timeline|roatingpaniting PlayFromStart)
      (:Update
        (Transformation|SetRelativeRotation (Variables|Default|Getpicture%20frame) (Math|Rotator|MakeRotator 0.0 (Math|Float|Lerp (.pitch (Variables|Default|GetstartingRo)) (- (.pitch (Variables|Default|GetstartingRo)) 9e+01) _rotation) 0.0) false false))
      (:Finished
        (Variables|Default|SetstartingRo (Math|Rotator|MakeRotator 0.0 (Math|Float|Lerp (.pitch (Variables|Default|GetstartingRo)) (- (.pitch (Variables|Default|GetstartingRo)) 9e+01) _rotation) 0.0))
        (Variables|Default|Setframemoving false)
        (bind _result (Math|Integer|IncrementInt (Variables|Default|Getframeposition))
          (:%20%20
            (bind _output_get (Variables|Default|Setframeposition _result))
            (if (> _output_get 3)
              (Variables|Default|Setframeposition 0)
              (elif (== 3 (Variables|Default|Getframeposition))
                (Default|CallEvdPuzzlefailed)
                (elif (== (Variables|Default|GetpuzzleSolved) (Variables|Default|Getframeposition))
                  (Default|CallEvdPuzzlebeat))))))))))

(event EventBeginPlay
  (Variables|Default|SetstartingRo (Variables|/Script/Engine.SceneComponent|GetRelativeRotation (Variables|Default|Getpicture%20frame))))

(event EventInteractEvent
  (params (Interactor :type Actor%20Object%20Reference))
  (Utilities|Casting|CastToBP_C_Game Interactor)
  (CallFunction|Roataed))

(fn ConstructionScript
  (|CallParentFunction))