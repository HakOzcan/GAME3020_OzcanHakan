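; BP_ComputerInteraction is an interactable computer that hands its Passcode to the interacting BP_C_Game.
; Interaction focus toggles custom depth on the Computer component for highlighting.
; Entering the Box trigger shows one widget at once and a code widget after a delay, and leaving hides both.
; The overlap is unfiltered, and leaving does not cancel a pending delayed reveal.
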(event OnComponentBeginOverlap(Box)
  (params (OverlappedComponent :type Primitive%20Component%20Object%20Reference) (OtherActor :type Actor%20Object%20Reference) (OtherComp :type Primitive%20Component%20Object%20Reference) (OtherBodyIndex :type Integer) (bFromSweep :type Boolean) (SweepResult :type Hit%20Result%20Structure%20%28by%20ref%29))
  (Development|SetHiddeninGame (Variables|Default|GetWidget) false false)
  (Utilities|FlowControl|Delay 5.0)
  (Development|SetHiddeninGame (Variables|Default|GetCodewidget) false false))

(event OnComponentEndOverlap(Box)
  (params (OverlappedComponent :type Primitive%20Component%20Object%20Reference) (OtherActor :type Actor%20Object%20Reference) (OtherComp :type Primitive%20Component%20Object%20Reference) (OtherBodyIndex :type Integer))
  (Development|SetHiddeninGame (Variables|Default|GetWidget) true false)
  (Development|SetHiddeninGame (Variables|Default|GetCodewidget) true false))

(event EventBeginPlay)

(event Collision|EventActorBeginOverlap
  (params (OtherActor :type Actor%20Object%20Reference)))

(event EventTick
  (params (DeltaSeconds :type Float%20%28single-precision%29)))

(event EventInteractEvent
  (params (Interactor :type Actor%20Object%20Reference))
  (bind _asbp_c_game (Utilities|Casting|CastToBP_C_Game Interactor))
  (Default|SetPlayerPasscode _asbp_c_game (Variables|Default|GetPasscode)))

(event EventToggleInteractFocus
  (params (focus :type Boolean))
  (Rendering|SetRenderCustomDepth (Variables|Default|GetComputer) focus))

(fn ConstructionScript)