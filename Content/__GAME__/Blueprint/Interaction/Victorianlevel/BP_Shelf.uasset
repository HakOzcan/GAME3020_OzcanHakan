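; BP_Shelf is a Victorian-level interaction prop: a shelf whose books fall off when something overlaps its trigger box.
; On the first Box overlap, a DoOnce enables physics simulation on the ten book and static mesh components.
; It then pushes them all with the same fixed impulse along negative X and plays a collapse sound at the actor's location.
; An AddForce node is left unconnected and never runs.
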(event OnComponentBeginOverlap(Box)
  (params (OverlappedComponent :type Primitive%20Component%20Object%20Reference) (OtherActor :type Actor%20Object%20Reference) (OtherComp :type Primitive%20Component%20Object%20Reference) (OtherBodyIndex :type Integer) (bFromSweep :type Boolean) (SweepResult :type Hit%20Result%20Structure%20%28by%20ref%29))
  (Utilities|FlowControl|DoOnce false
    (:Completed
      (Physics|SetSimulatePhysics (Variables|Default|GetMesh_Book2) true)
      (Physics|AddImpulse (Variables|Default|GetStaticMesh7) "-400.000000,0.000000,0.000000" "None" false)
      (Audio|PlaySoundatLocation "/Game/__GAME__/Audio/collapse.collapse" (Transformation|GetActorLocation) "0, 0, 0" 1.0 1.0 0.0 0 0 0 0))))

(event EventBeginPlay)

(event Collision|EventActorBeginOverlap
  (params (OtherActor :type Actor%20Object%20Reference)))

(event EventTick
  (params (DeltaSeconds :type Float%20%28single-precision%29)))

(fn ConstructionScript)