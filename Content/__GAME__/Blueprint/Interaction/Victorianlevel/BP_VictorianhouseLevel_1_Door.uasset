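; Door actor for Victorian house level 1 that swings by timeline-driven yaw when a BP_C_Game actor enters or leaves its trigger box.
; Begin overlap drives the DoorOpen timeline; end overlap drives a second timeline after a two-second delay.
; Each passes through a FlipFlop, so alternate triggers stop the timeline instead of playing it.
; An OPenDoor event also plays DoorOpen directly, while the door sounds are unconnected.
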(event OnComponentEndOverlap(Box)
  (params (OverlappedComponent :type Primitive%20Component%20Object%20Reference) (OtherActor :type Actor%20Object%20Reference) (OtherComp :type Primitive%20Component%20Object%20Reference) (OtherBodyIndex :type Integer))
  (Utilities|Casting|CastToBP_C_Game OtherActor)
  (Utilities|FlowControl|Delay 2.0)
  (Utilities|FlowControl|FlipFlop
    (:A
      (bind _newtrack_0 (Timeline|Timeline PlayFromStart)
        (:Update
          (Transformation|SetRelativeRotation (Variables|Default|GetDoor) (Math|Rotator|MakeRotator 0.0 0.0 _newtrack_0) false false))))
    (:B
      (Timeline|Timeline Stop))))

(event OnComponentBeginOverlap(Box)
  (params (OverlappedComponent :type Primitive%20Component%20Object%20Reference) (OtherActor :type Actor%20Object%20Reference) (OtherComp :type Primitive%20Component%20Object%20Reference) (OtherBodyIndex :type Integer) (bFromSweep :type Boolean) (SweepResult :type Hit%20Result%20Structure%20%28by%20ref%29))
  (Utilities|Casting|CastToBP_C_Game OtherActor)
  (Utilities|FlowControl|FlipFlop
    (:A
      (bind _newtrack_0 (Timeline|DoorOpen PlayFromStart)
        (:Update
          (Transformation|SetRelativeRotation (Variables|Default|GetDoor) (Math|Rotator|MakeRotator 0.0 0.0 _newtrack_0) false false))))
    (:B
      (Timeline|DoorOpen Stop))))

(event Custom|OPenDoor
  (bind _newtrack_0 (Timeline|DoorOpen Play)
    (:Update
      (Transformation|SetRelativeRotation (Variables|Default|GetDoor) (Math|Rotator|MakeRotator 0.0 0.0 _newtrack_0) false false))))

(event EventBeginPlay)

(event Collision|EventActorBeginOverlap
  (params (OtherActor :type Actor%20Object%20Reference)))

(event EventTick
  (params (DeltaSeconds :type Float%20%28single-precision%29)))

(fn ConstructionScript)