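; BP_NoteMaker is an interactable note that the player can read when nearby.
; Actor overlap enables input and copies its Notecard value to the player character's NoteCardIndex; leaving disables input and removes the letter display.
; While input is enabled, the gamepad left face button toggles the LetterDisplay widget through a FlipFlop.
; A separate Box overlap shows or hides two widget components and plays an eerie 2D sound on entry.
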(event OnComponentBeginOverlap(Box)
  (params (OverlappedComponent :type Primitive%20Component%20Object%20Reference) (OtherActor :type Actor%20Object%20Reference) (OtherComp :type Primitive%20Component%20Object%20Reference) (OtherBodyIndex :type Integer) (bFromSweep :type Boolean) (SweepResult :type Hit%20Result%20Structure%20%28by%20ref%29))
  (Rendering|SetVisibility (Variables|Default|GetWidget) true false)
  (Rendering|SetVisibility (Variables|Default|GetNotewidget) true false)
  (Audio|PlaySound2D "/Game/__GAME__/Audio/scary-spooky-eerie-suspense-283845.scary-spooky-eerie-suspense-283845" 1.0 1.0 0.0 0 0))

(event OnComponentEndOverlap(Box)
  (params (OverlappedComponent :type Primitive%20Component%20Object%20Reference) (OtherActor :type Actor%20Object%20Reference) (OtherComp :type Primitive%20Component%20Object%20Reference) (OtherBodyIndex :type Integer))
  (Rendering|SetVisibility (Variables|Default|GetWidget) false false)
  (Rendering|SetVisibility (Variables|Default|GetNotewidget) false false))

(event EventBeginPlay)

(event EventTick
  (params (DeltaSeconds :type Float%20%28single-precision%29)))

(event Collision|EventActorBeginOverlap
  (params (OtherActor :type Actor%20Object%20Reference))
  (Input|EnableInput (Game|GetPlayerController 0))
  (bind _asbp_c_game (Utilities|Casting|CastToBP_C_Game (Game|GetPlayerCharacter 0)))
  (Variables|/Game/__GAME__/Blueprint/Game_Essential/BP_C_Game.BP_C_Game_C|SetNoteCardIndex _asbp_c_game (Variables|Default|Getnotecard)))

(event Collision|EventActorEndOverlap
  (params (OtherActor :type Actor%20Object%20Reference))
  (Input|DisableInput 0)
  (Widget|RemovefromParent (stale Input|GamepadEvents|GamepadFaceButtonLeft _returnvalue)))

(event Input|GamepadEvents|GamepadFaceButtonLeft
  (params (Key :type Key%20Structure))
  (:Pressed
    (Utilities|FlowControl|FlipFlop
      (:A
        (bind _returnvalue (UserInterface|CreateWidget "/Game/__GAME__/Blueprint/Interaction/Interaction_UI/LetterDisplay.LetterDisplay_C"))
        (UserInterface|Viewport|AddtoViewport _returnvalue 0))
      (:B
        (Widget|RemovefromParent _returnvalue)))))

(fn ConstructionScript)