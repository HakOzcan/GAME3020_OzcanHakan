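; BP_Door is a keypad door actor with a trigger box that enables input while a BP_C_Game actor overlaps it.
; Gamepad left face button flip-flops between showing a Numpad widget for a newly created player and clearing all widgets, as leaving the box also does.
; OpenDoor, not called in this graph, slides the door by timeline.
; InteractEvent is empty; passcode checking and rotation logic are disconnected.
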(event OnComponentEndOverlap(Box)
  (params (OverlappedComponent :type Primitive%20Component%20Object%20Reference) (OtherActor :type Actor%20Object%20Reference) (OtherComp :type Primitive%20Component%20Object%20Reference) (OtherBodyIndex :type Integer))
  (bind _returnvalue (Game|GetPlayerController 0))
  (Utilities|Casting|CastToBP_C_Game OtherActor)
  (Input|DisableInput (Game|GetPlayerController 0))
  (Viewport|RemoveAllWidgets)
  (Input|SetInputModeGameOnly _returnvalue false)
  (Variables|/Script/Engine.PlayerController|SetbShowMouseCursor _returnvalue false))

(event OnComponentBeginOverlap(Box)
  (params (OverlappedComponent :type Primitive%20Component%20Object%20Reference) (OtherActor :type Actor%20Object%20Reference) (OtherComp :type Primitive%20Component%20Object%20Reference) (OtherBodyIndex :type Integer) (bFromSweep :type Boolean) (SweepResult :type Hit%20Result%20Structure%20%28by%20ref%29))
  (Utilities|Casting|CastToBP_C_Game OtherActor)
  (Input|EnableInput (Game|GetPlayerController 0)))

(event Custom|Open%20Door
  (bind _newtrack_4 (Timeline|Timeline_0 Play)
    (:Update
      (Transformation|SetRelativeLocation (Variables|Default|GetDoor) _newtrack_4 false false)
      (Input|SetInputModeGameandUI (Game|GetPlayerController 0) 0 "DoNotLock" true false)
      (switch string (Game|GetPlatformName)))))

(event EventBeginPlay)

(event Collision|EventActorBeginOverlap
  (params (OtherActor :type Actor%20Object%20Reference)))

(event EventTick
  (params (DeltaSeconds :type Float%20%28single-precision%29)))

(event EventInteractEvent
  (params (Interactor :type Actor%20Object%20Reference)))

(event Input|GamepadEvents|GamepadFaceButtonLeft
  (params (Key :type Key%20Structure :default "None"))
  (bind _returnvalue (Game|GetPlayerController 0))
  (:Pressed
    (Utilities|FlowControl|FlipFlop
      (:A
        (bind _returnvalue_2 (Class|GameplayStatics|CreatePlayer (Class|MyBlueprintFunctionLibrary|GetActiveControllerID)))
        (bind _returnvalue_3 (UserInterface|CreateWidget "/Game/__GAME__/Blueprint/Interaction/Interaction_UI/Numpad.Numpad_C" _returnvalue_2))
        (UserInterface|Viewport|AddtoViewport _returnvalue_3 0)
        (Input|SetInputModeUIOnly _returnvalue 0 "DoNotLock" false))
      (:B
        (Viewport|RemoveAllWidgets)
        (Input|SetInputModeGameOnly _returnvalue false)
        (Variables|/Script/Engine.PlayerController|SetbShowMouseCursor _returnvalue false)))))

(fn ConstructionScript)