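; Spotlight actor that flickers at irregular intervals between a low intensity and a normal one.
; BeginPlay starts an endless loop that waits a random time between Min and Max on a retriggerable delay.
; After each wait, a FlipFlop sets the SpotLightComponent to MinFlickerIntensity or Intensity in turn, then re-enters the delay, so no Tick is used.
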(event EventBeginPlay
  (Utilities|FlowControl|RetriggerableDelay (Math|Random|RandomFloatinRange (Variables|Default|GetMin) (Variables|Default|GetMax)) :!label _label)
  (Utilities|FlowControl|FlipFlop
    (:A
      (Rendering|Components|Light|SetIntensity (Variables|Default|GetSpotLightComponent) (Variables|Default|GetMinFlickerIntensity))
      (goto _label))
    (:B
      (Rendering|Components|Light|SetIntensity (Variables|Default|GetSpotLightComponent) (Variables|Default|GetIntensity))
      (goto _label))))

(event EventTick
  (params (DeltaSeconds :type Float%20%28single-precision%29)))

(fn ConstructionScript)